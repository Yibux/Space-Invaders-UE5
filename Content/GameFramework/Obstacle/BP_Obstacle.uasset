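; BP_Obstacle is a destructible obstacle actor that loses one health point per projectile hit.
; When health reaches zero, the HitByProjectile event destroys the actor.
; Otherwise, it creates a dynamic material instance from the Obstacle component's material and sets its ObstacleColor parameter.
; An inverted range normalization of health drives the color lerp, shifting from red toward near-white as health drops.
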(event Custom|HitByProjectile
  (bind _obstacle (Variables|Default|Getobstacle))
  (bind _output_get (Variables|Default|SetHealth (- (Variables|Default|GetHealth) 1)))
  (if (== _output_get 0)
    (Actor|DestroyActor)
    (else
      (bind _returnvalue (Rendering|Material|CreateDynamicMaterialInstance _obstacle 0 (Rendering|Material|GetMaterial _obstacle 0) "None" :!class /Script/Engine.PrimitiveComponent))
      (Rendering|Material|SetVectorParameterValue _returnvalue "ObstacleColor" (Math|Color|Lerp(LinearColor) "(R=1.000000,G=0.000000,B=0.007332,A=1.000000)" "(R=0.943928,G=0.939164,B=1.000000,A=1.000000)" (Math|Float|NormalizetoRange (Math|Conversions|ToFloat(Integer) (Variables|Default|GetHealth)) 6.0 0.0)) :!class /Script/Engine.MaterialInstanceDynamic))))

(fn ConstructionScript)