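; BP_BetterEnemy is a Space Invaders enemy that circles its spawn point in the YZ plane while firing projectiles.
; Tick derives the orbit position from an accumulating angle, and a self-recalling FireProjectile event randomly spawns shots at random intervals after an initial delay.
; Each projectile hit reduces health and may drop a health or shield power-up.
; At zero health it may drop another, destroys itself and notifies BP_SpaceInvadersGameMode of the kill.
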(event Custom|HandleDeath
  (if (Math|Random|RandomBool)
    (CallFunction|SpawnPowerUp))
  (Actor|DestroyActor)
  (bind _asbp_space_invaders_game_mode (Utilities|Casting|CastToBP_SpaceInvadersGameMode (Game|GetGameMode)))
  (Default|EnemyKilled _asbp_space_invaders_game_mode))

(event Custom|SpawnPowerUp
  (bind _cube (Variables|Default|GetCube))
  (bind _returnvalue (Transformation|GetWorldLocation _cube))
  (switch int (Math|Random|RandomIntegerinRange 0 1)
    (:Default
      (Game|SpawnActorfromClass "/Game/GameFramework/PowerUps/BP_PowerUpHealth.BP_PowerUpHealth_C" (Math|Transform|MakeTransform _returnvalue "0, 0, 0" "1.000000,1.000000,1.000000") "Undefined" "MultiplyWithRoot" 0 0 :!label _label))
    (:0
      (goto _label))
    (:1
      (Game|SpawnActorfromClass "/Game/GameFramework/PowerUps/BP_PowerUpShield.BP_PowerUpShield_C" (Math|Transform|MakeTransform _returnvalue "0, 0, 0" "1.000000,1.000000,1.000000") "Undefined" "MultiplyWithRoot" 0 0))))

(event Custom|HitByProjectile
  (bind _output_get (Variables|Default|SetHealth (- (Variables|Default|GetHealth) 1)))
  (if (Math|Random|RandomBool)
    (CallFunction|SpawnPowerUp))
  (if (== _output_get 0)
    (CallFunction|HandleDeath)))

(event Custom|FireProjectile
  (if (Math|Random|RandomBool)
    (Game|SpawnActorfromClass "/Game/GameFramework/Enemy/BP_EnemyProjectile.BP_EnemyProjectile_C" (Math|Transform|MakeTransform (Transformation|GetWorldLocation (Variables|Default|GetEnemyProjectileSpawnLocation)) "0, 0, 0" "1.000000,1.000000,1.000000") "Undefined" "MultiplyWithRoot" 0 0))
  (Utilities|FlowControl|Delay (Math|Random|RandomFloatinRange 0.2 1.0))
  (CallFunction|FireProjectile))

(event EventBeginPlay
  (Variables|Default|SetPivotLocation (Transformation|GetActorLocation))
  (Utilities|FlowControl|Delay (Math|Random|RandomFloatinRange 1.0 2.0))
  (CallFunction|FireProjectile))

(event EventTick
  (params (DeltaSeconds :type Float%20%28single-precision%29))
  (bind _radius (Variables|Default|GetRadius))
  (Variables|Default|SetAngle (+ (Variables|Default|GetAngle) (* (Utilities|Time|GetWorldDeltaSeconds) (Variables|Default|GetRotationSpeed))))
  (bind _output_get (Variables|Default|SetPivotLocation (Math|Vector|MakeVector (.x (Variables|Default|GetPivotLocation)) (.y (Variables|Default|GetPivotLocation)) (.z (Variables|Default|GetPivotLocation)))))
  (Transformation|SetActorLocation (+ _output_get (Math|Vector|MakeVector 0.0 (* (Math|Trig|Sin(Radians) (Variables|Default|GetAngle)) _radius) (* _radius (Math|Trig|Cos(Radians) (Variables|Default|GetAngle))))) false false))

(fn ConstructionScript)