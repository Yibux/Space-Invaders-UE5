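; Space Invaders-style enemy that sweeps along the Y axis, gradually speeding up to a cap and reversing at fixed bounds.
; After a random startup delay, a self-repeating timed event randomly fires projectiles from its spawn point.
; HandleDeath randomly drops a health or shield power-up, favoring health, then destroys the actor and notifies BP_SpaceInvadersGameMode of the kill.
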(event Custom|HandleDeath
  (bind _cube (Variables|Default|GetCube))
  (bind _returnvalue (Transformation|GetWorldLocation _cube))
  (if (Math|Random|RandomBool)
    (switch int (Math|Random|RandomIntegerinRange 0 2)
      (:Default
        (Game|SpawnActorfromClass "/Game/GameFramework/PowerUps/BP_PowerUpHealth.BP_PowerUpHealth_C" (Math|Transform|MakeTransform _returnvalue "0, 0, 0" "1.000000,1.000000,1.000000") "Undefined" "MultiplyWithRoot" 0 0 :!label _label))
      (:0
        (goto _label))
      (:1
        (Game|SpawnActorfromClass "/Game/GameFramework/PowerUps/BP_PowerUpShield.BP_PowerUpShield_C" (Math|Transform|MakeTransform _returnvalue "0, 0, 0" "1.000000,1.000000,1.000000") "Undefined" "MultiplyWithRoot" 0 0))))
  (Actor|DestroyActor)
  (bind _asbp_space_invaders_game_mode (Utilities|Casting|CastToBP_SpaceInvadersGameMode (Game|GetGameMode)))
  (Default|EnemyKilled _asbp_space_invaders_game_mode))

(event Custom|FireProjectile
  (if (Math|Random|RandomBool)
    (Game|SpawnActorfromClass "/Game/GameFramework/Enemy/BP_EnemyProjectile.BP_EnemyProjectile_C" (Math|Transform|MakeTransform (Transformation|GetWorldLocation (Variables|Default|GetEnemyProjectileSpawnLocation)) "0, 0, 0" "1.000000,1.000000,1.000000") "Undefined" "MultiplyWithRoot" 0 0))
  (Utilities|FlowControl|Delay (Math|Random|RandomFloatinRange 2.0 5.0))
  (CallFunction|FireProjectile))

(event EventBeginPlay
  (Utilities|FlowControl|Delay (Math|Random|RandomFloatinRange 1.0 2.0))
  (CallFunction|FireProjectile))

(event EventTick
  (params (DeltaSeconds :type Float%20%28single-precision%29))
  (bind _enemyprojectilespawnlocation (Variables|Default|GetEnemyProjectileSpawnLocation))
  (bind _returnvalue (Transformation|GetWorldLocation _enemyprojectilespawnlocation))
  (Variables|Default|SetSpeed (Math|Float|Clamp(Float) (+ (Variables|Default|GetSpeed) 0.1) 2.0 (Variables|Default|GetMaxSpeed)))
  (if (or (>= (.y _returnvalue) 5.2e+02) (<= (.y _returnvalue) -1.08e+03))
    (Variables|Default|SetDirection (* (Variables|Default|GetDirection) -1.0)))
  (Transformation|AddActorWorldOffset (Math|Vector|MakeVector 0.0 (* (Variables|Default|GetDirection) (Variables|Default|GetSpeed)) 0.0)))

(fn ConstructionScript)