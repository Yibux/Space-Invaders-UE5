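; BP_MyProjectile is a projectile that damages or kills what it hits and awards the player points.
; Its capsule overlap event runs a Sequence of casts to tell obstacles, enemies and better enemies apart.
; Obstacles and better enemies handle the hit themselves, while basic enemies die outright, and both enemy types add score through BP_PlayerPawn.
; All three branches share one DestroyActor call that removes the projectile.
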(event OnComponentBeginOverlap(Capsule)
  (params (OverlappedComponent :type Primitive%20Component%20Object%20Reference) (OtherActor :type Actor%20Object%20Reference) (OtherComp :type Primitive%20Component%20Object%20Reference) (OtherBodyIndex :type Integer) (bFromSweep :type Boolean) (SweepResult :type Hit%20Result%20Structure%20%28by%20ref%29))
  (bind _returnvalue (Game|Player|GetPlayerPawn 0))
  (Utilities|FlowControl|Sequence
    (:then_0
      ;[0.15 0.15 0.15 0.5] Check if obstacle is hit then decrease health
      (bind _asbp_obstacle (Utilities|Casting|CastToBP_Obstacle OtherActor))
      (Default|HitbyProjectile _asbp_obstacle))
    (:then_1
      ;[0.15 0.15 0.15 0.5] Destroy Enemy if hit
      (bind _asbp_enemy (Utilities|Casting|CastToBP_Enemy OtherActor))
      (Default|HandleDeath _asbp_enemy)
      (bind _asbp_player_pawn (Utilities|Casting|CastToBP_PlayerPawn _returnvalue))
      (Default|UpdateScore _asbp_player_pawn 10))
    (:then_2
      (bind _asbp_better_enemy (Utilities|Casting|CastToBP_BetterEnemy OtherActor))
      (Default|HitbyProjectile _asbp_better_enemy)
      (bind _asbp_player_pawn_2 (Utilities|Casting|CastToBP_PlayerPawn _returnvalue))
      (Default|UpdateScore _asbp_player_pawn_2 25)))
  (Actor|DestroyActor))

(fn ConstructionScript)